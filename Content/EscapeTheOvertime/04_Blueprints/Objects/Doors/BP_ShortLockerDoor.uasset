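; BP_ShortLockerDoor is a short locker door that vanishes with an opening sound when something overlaps its box.
; On BeginPlay it rotates its child actor using the actor's rotation and lowers it for bottom doors, identified by a roll of 180 or more.
; The box overlap, unfiltered by actor type, destroys the rect light and cube rather than animating them, playing the cabinet cue once.
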(event `self.ReceiveBeginPlay`
  (bind (_returnvalue_location _returnvalue_rotation) (`KismetMathLibrary.BreakTransform` (`self.GetTransform`)))
  (bind _returnvalue_roll (`KismetMathLibrary.BreakRotator` (`self.K2_GetActorRotation`)))
  (`SceneComponent.K2_SetRelativeRotation` (`self.ChildActor`) _returnvalue_rotation false false)
  (if (>= _returnvalue_roll 180.0)
    (`SceneComponent.K2_AddWorldTransform` (`self.ChildActor`) (`KismetMathLibrary.MakeTransform` (0.0 0.0 -100.0)) false false)))

(event `self.BoxComp.OnComponentBeginOverlap`
  (params (OverlappedComponent :type "PrimitiveComponent Object Reference") (OtherActor :type "Actor Object Reference") (OtherComp :type "PrimitiveComponent Object Reference") (OtherBodyIndex :type Integer) (bFromSweep :type Boolean) (SweepResult :type "HitResult Structure (by ref)"))
  (bind _cube (`self.Cube`))
  (bind _rectlight (`self.RectLight`))
  (`/Engine/EditorBlueprintResources/StandardMacros.IsValid` _rectlight
    (:`Is Valid`
      (`ActorComponent.K2_DestroyComponent` _rectlight))
    (:`Is Not Valid`
      _))
  (`/Engine/EditorBlueprintResources/StandardMacros.IsValid` _cube
    (:`Is Valid`
      (`ActorComponent.K2_DestroyComponent` _cube)
      (`/Engine/EditorBlueprintResources/StandardMacros.DoOnce` false
        (:`Completed`
          (`GameplayStatics.PlaySoundAtLocation` "/Game/EscapeTheOvertime/06_Audio/SFX/Environment/DoorOpen/OPEN_Cabinet_Cue.OPEN_Cabinet_Cue" (`self.K2_GetActorLocation`) (struct) 1.0 1.0 0.0 null null null null))))))

(fn `UserConstructionScript`)